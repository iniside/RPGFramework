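; BP_RPGHUD is a HUD Blueprint that draws an RPG character's health values on screen as debug-style text.
; Each DrawHUD call casts the HUD hit actor to RPGCharacter and draws its Health and labelled MaxHealth attributes with canvas DrawText, placing the latter at half screen width.
; Tick and the construction script are empty, and the CharOwner variable is unused.
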(event `self.ReceiveDrawHUD`
  (params (SizeX :type Integer) (SizeY :type Integer))
  (bind _returnvalue (`self.GetHUDHitActor`))
  (bind _asrpgcharacter (cast `RPGCharacter` _returnvalue))
  (bind _attributes (`RPGCharacter.Attributes` _asrpgcharacter))
  (`self.DrawText` (`KismetStringLibrary.Conv_DoubleToString` (`RPGAttributeComponent.Health` _attributes)) (struct :`R` 0.982517 :`B` 1.0 :`A` 1.0) 0.0 0.0 null 3.0)
  (`self.DrawText` (`KismetStringLibrary.BuildString_Double` "" "Max Heahlth" (`RPGAttributeComponent.MaxHealth` _attributes)) (struct :`R` 1.0 :`B` 0.160202 :`A` 1.0) (`KismetMathLibrary.Conv_IntToDouble` (/ SizeX 2)) 0.0 null 4.0))

(event `self.ReceiveTick`
  (params (DeltaSeconds :type "Float (single-precision)")))

(fn `UserConstructionScript`)