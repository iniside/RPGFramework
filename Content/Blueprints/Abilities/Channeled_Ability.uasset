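; Channeled ability that applies repeating fire spell damage with a LifeSteal periodic effect to the actor hit from the weapon socket.
; On start, a fraction of the owner's Intelligence feeds SpellDamage and FireDamage calculations to set the Health value of an instant DamagePure effect.
; That effect is nested in a timed periodic effect on the hit actor.
; Trail FX, direct damage, effect-modifier and debug counter branches are disconnected.
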(event `self.OnAbilityStart`
  (bind _abilityowner (`self.AbilityOwner`))
  (bind _hitactor (`self.HitActor`))
  (bind _returnvalue (`self.GetHitResult` 10000.0 "WeaponSocket"))
  (set `self.HitActor` (`.HitActor` (`GameplayStatics.BreakHitResult` _returnvalue)))
  (bind _returnvalue_2 (`RPGAttributeComponent.AttributeOperation` (`self.OwnerAttributeComp`) "Intelligence" 5.0 "Attribute_Divide"))
  (bind _returnvalue_3 (`RPGEffectBPLibrary.CreatePeriodicEffect` (`self.HitActor`) (`self.AbilityOwner`) "/Game/Blueprints/Effects/LifeSteal.LifeSteal_C" 1.0 8.0))
  (bind _returnvalue_4 (`DamagefunctionStatics.FireDamage` _hitactor _abilityowner (`DamagefunctionStatics.SpellDamage` _hitactor _abilityowner _returnvalue_2)))
  (bind _returnvalue_5 (`RPGEffectBPLibrary.CreateInstantEffect` (`self.HitActor`) (`self.AbilityOwner`) "/Game/Blueprints/Effects/DamagePure.DamagePure_C" (`|MakeArray` (make `ModdableAttributes` "Health" _returnvalue_4)) "Health" _returnvalue_4))
  (`RPGEffectBPLibrary.ApplyPeriodicEffect` _returnvalue_3 (`|MakeArray` _returnvalue_5 :!type "RPGEffectBase Object Reference")))