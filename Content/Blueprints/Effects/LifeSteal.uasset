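; LifeSteal is an effect Blueprint that damages its target and heals the effect's causer.
; On application and on each period, it applies one DamagePure effect to Target and one HealEffect to CausedBy.
; Both child effects are built from the same AttributeSpecList, passed through unchanged.
; Unconnected debug print and radial-apply nodes remain in the graph but never run.
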(event `self.OnEffectAppiled`
  (bind _attributespeclist (`self.AttributeSpecList`))
  (bind _causedby (`self.CausedBy`))
  (`RPGEffectBPLibrary.ApplyEffect` (`self.Target`) _causedby 1 (make `RPGEffectBase.EffectSpec` _attributespeclist "/Game/Blueprints/Effects/DamagePure.DamagePure_C" (struct) (struct)) :!label _label)
  (`RPGEffectBPLibrary.ApplyEffect` _causedby _causedby 1 (make `RPGEffectBase.EffectSpec` _attributespeclist "/Game/Blueprints/Effects/HealEffect.HealEffect_C" (struct) (struct))))

(event `self.OnEffectPeriod`
  (goto _label))