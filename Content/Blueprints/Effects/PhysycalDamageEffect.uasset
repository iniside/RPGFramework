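; Physical damage effect that lowers the target's Health, reduced by the target's toughness.
; When applied, it loops through the attributes to modify, takes each Health entry and subtracts the target's "Thoughness" value from its mod value.
; The result is subtracted from Health through the target's attributes with no clamp, so toughness above the damage yields a negative subtraction.
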(event `self.OnEffectAppiled`
  (bind _targetattributes (`self.TargetAttributes`))
  (for _array_element (`self.AttributesToModify`)
    (bind (_attributename _modvalue) (break `ModdableAttributes` _array_element))
    (if (== _attributename "Health")
      (bind _returnvalue (`RPGAttributeComponent.GetNumericValue` _targetattributes "Thoughness"))
      (`RPGAttributeComponent.ModifyAttribute` _targetattributes (make `ModdableAttributes` _attributename (- _modvalue _returnvalue)) "Attribute_Subtract"))))