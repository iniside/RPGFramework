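; Test ability that applies a life-steal effect to whatever actor its owner hits.
; On ability start it gets a long-range hit result from the weapon socket and applies one LifeStealEffect to the hit actor, with the ability owner as causer.
; An unconnected MakeEffectSpec node holds an inline LifeSteal spec with tag-targeted Health modifiers for damage and heal.
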(event `self.OnAbilityStart`
  (bind _returnvalue (`self.GetHitResult` 10000.0 "WeaponSocket"))
  (`RPGEffectBPLibrary.ApplyEffect` (`.HitActor` (`GameplayStatics.BreakHitResult` _returnvalue)) (`self.AbilityOwner`) 1 (`self.LifeStealEffect`)))