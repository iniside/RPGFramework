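; RPG_GenericEffect is an effect Blueprint that subtracts fixed amounts of Health and Energy from its target when applied.
; The applied event makes a single ModifyTargetAttributes call using the subtract operation, while the periodic event does nothing.
; Disconnected leftovers include bindings to empty received-effect handlers, a radius-based LifeSteal spread to multiple targets, and debug prints, none of which run.
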(event `self.OnEffectAppiled`
  (`self.ModifyTargetAttributes` (`|MakeArray` (make `ModdableAttributes` "Health" 30.0) (make `ModdableAttributes` "Energy" 20.0)) "Attribute_Subtract"))

(event `self.OnEffectPeriod`)

(event `OnRecivedEffect_EventOMG`
  (params (WhoRecievedEffect :type "Actor Object Reference") (Effect :type "RPGEffectBase Class Reference")))

(event `OnRecivedEffect_Event`
  (params (WhoRecievedEffect :type "Actor Object Reference") (Effect :type "RPGEffectBase Class Reference")))